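; GM_Manager is a game manager that handles player respawn, win and loss results, and pausing.
; On BeginPlay it caches the player's BP_HUD, which it later uses to display the death or victory message.
; Respawn spawns and possesses a new BP_Player at a stored transform while the passed-in lives count is above zero, otherwise reporting death.
; PauseGame toggles the paused state through a FlipFlop.
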(event `self.ReceiveBeginPlay`
  (bind _asbp_hud (cast `/Game/Game/GameBP/BP_HUD` (`PlayerController.GetHUD` (`GameplayStatics.GetPlayerController` 0))))
  (set `self. HUD` _asbp_hud))

(event `Respawn`
  (params (Lifes :type Integer))
  ; Respawn Player
  (if (> Lifes 0)
    (bind _returnvalue (`|SpawnActorFromClass` "/Game/Game/Player/BP_Player.BP_Player_C" (`self.SpawnTransform`) "Undefined" "MultiplyWithRoot" null null))
    (`Controller.Possess` (`GameplayStatics.GetPlayerController` 0) _returnvalue)
    (else
      (`/Game/Game/GameBP/BP_HUD.GameResult` (`self. HUD`) "YOU DIED"))))

(event `PlayerWin`
  (`/Game/Game/GameBP/BP_HUD.GameResult` (`self. HUD`) "ACABOOOO"))

(event `PauseGame`
  (`/Engine/EditorBlueprintResources/StandardMacros.FlipFlop`
    (:`A`
      (`GameplayStatics.SetGamePaused` true))
    (:`B`
      (`GameplayStatics.SetGamePaused` false))))

(fn `UserConstructionScript`)