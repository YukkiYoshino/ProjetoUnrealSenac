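; PC_Main is the player controller that handles input setup, player lives and the pause menu.
; BeginPlay adds the IMC_Player Enhanced Input mapping context and caches references to GM_Manager and BP_HUD.
; Each possessed pawn gets an OnDestroyed binding that decrements Lifes and passes it to the game mode's Respawn.
; The pause input and DisableMenu event share one path calling PauseGame on the game mode and PauseMenu on the HUD.
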(event `self.ReceiveBeginPlay`
  (`EnhancedInputSubsystemInterface.AddMappingContext` (pcsubsystem `EnhancedInputLocalPlayerSubsystem` self) "/Game/Game/Player/Inputs/IMC_Player.IMC_Player" 0 (struct))
  (bind _asgm_manager (cast `/Game/Game/GameBP/GM_Manager` (`GameplayStatics.GetGameMode`)))
  (set `self.GM` _asgm_manager)
  (bind _asbp_hud (cast `/Game/Game/GameBP/BP_HUD` (`self.GetHUD`)))
  (set `self.HUD` _asbp_hud))

(event `self.ReceivePossess`
  (params (PossessedPawn :type "Pawn Object Reference"))
  (add `self.OnDestroyed` PossessedPawn (delegate `OnDestroy_Event`)))

(event `OnDestroy_Event` :!signature `self.OnDestroyed`
  (params (DestroyedActor :type "Actor Object Reference"))
  (bind _result (`/Engine/EditorBlueprintResources/StandardMacros.DecrementInt` (`self.Lifes`))
    (:`  `
      (`/Game/Game/GameBP/GM_Manager.Respawn` (`self.GM`) _result))))

(event `DisableMenu`
  (`/Game/Game/GameBP/GM_Manager.PauseGame` (`self.GM`) :!label _label)
  (`/Game/Game/GameBP/BP_HUD.PauseMenu` (`self.HUD`)))

(event `EnhancedInput|/Game/Game/Player/Inputs/IA_PauseMenu`
  (params (ActionValue :type Boolean) (ElapsedSeconds :type "Float (double-precision)") (TriggeredSeconds :type "Float (double-precision)") (InputAction :type "InputAction Object Reference" :default "/Game/Game/Player/Inputs/IA_PauseMenu.IA_PauseMenu"))
  (:`Started`
    (goto _label)))

(fn `UserConstructionScript`)