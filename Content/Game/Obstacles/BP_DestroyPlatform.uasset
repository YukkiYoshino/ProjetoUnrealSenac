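; BP_DestroyPlatform is an obstacle platform that changes color with each overlap and destroys itself after the second.
; Each overlap on its Collision component increments an Index, with no filter on the overlapping actor.
; Tick reapplies the material from that Index, going from green to yellow to red, and at red a short Delay precedes DestroyActor.
; The construction script sets the initial green material.
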(event `self.ReceiveTick`
  (params (DeltaSeconds :type "Float (single-precision)"))
  (bind _plataform (`self.Plataform`))
  (if (== (`self.Index`) 0)
    (`PrimitiveComponent.SetMaterial` _plataform 0 "/Game/Game/Obstacles/Materials/M_Green.M_Green")
    (elif (== (`self.Index`) 1)
      (`PrimitiveComponent.SetMaterial` _plataform 0 "/Game/Game/Obstacles/Materials/M_Yellow.M_Yellow")
      (else
        (`PrimitiveComponent.SetMaterial` _plataform 0 "/Game/Game/Obstacles/Materials/M_Red.M_Red")
        (`KismetSystemLibrary.Delay` 1.5)
        (`self.K2_DestroyActor`)))))

(event `self.Collision.OnComponentBeginOverlap`
  (params (OverlappedComponent :type "PrimitiveComponent Object Reference") (OtherActor :type "Actor Object Reference") (OtherComp :type "PrimitiveComponent Object Reference") (OtherBodyIndex :type Integer) (bFromSweep :type Boolean) (SweepResult :type "HitResult Structure (by ref)"))
  (set `self.Index` (+ (`self.Index`) 1)))

(fn `UserConstructionScript`
  (`PrimitiveComponent.SetMaterial` (`self.Plataform`) 0 "/Game/Game/Obstacles/Materials/M_Green.M_Green"))