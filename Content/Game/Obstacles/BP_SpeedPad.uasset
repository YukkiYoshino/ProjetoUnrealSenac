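; BP_SpeedPad is an obstacle pad that speeds up or slows the player standing on it.
; A looping timer randomly switches it every few seconds between a green fast state at MaxSpeed and a red slow state at a fraction of it.
; Box overlap applies the current speed to BP_Player's MaxWalkSpeed only on entry, and exit restores a hard-coded default.
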(event `self.Box.OnComponentBeginOverlap`
  (params (OverlappedComponent :type "PrimitiveComponent Object Reference") (OtherActor :type "Actor Object Reference") (OtherComp :type "PrimitiveComponent Object Reference") (OtherBodyIndex :type Integer) (bFromSweep :type Boolean) (SweepResult :type "HitResult Structure (by ref)"))
  (bind _asbp_player (cast `/Game/Game/Player/BP_Player` OtherActor))
  (set `CharacterMovementComponent.MaxWalkSpeed` (`self.Current Velocity`) (`Character.CharacterMovement` _asbp_player)))

(event `self.Box.OnComponentEndOverlap`
  (params (OverlappedComponent :type "PrimitiveComponent Object Reference") (OtherActor :type "Actor Object Reference") (OtherComp :type "PrimitiveComponent Object Reference") (OtherBodyIndex :type Integer))
  (bind _asbp_player (cast `/Game/Game/Player/BP_Player` OtherActor))
  (set `CharacterMovementComponent.MaxWalkSpeed` 300.0 (`Character.CharacterMovement` _asbp_player)))

(event `self.ReceiveBeginPlay`
  (`KismetSystemLibrary.K2_SetTimerDelegate` (delegate `ChangePad`) 3.0 true)
  (set `self.Current Velocity` (`self.MaxSpeed`)))

(event `ChangePad`
  (bind _pad (`self.Pad`))
  (if (`KismetMathLibrary.RandomBoolWithWeight` 0.5)
    (`PrimitiveComponent.SetMaterial` _pad 0 "/Game/Game/Obstacles/Materials/M_Green.M_Green")
    (set `self.Current Velocity` (`self.MaxSpeed`))
    (else
      (`PrimitiveComponent.SetMaterial` _pad 0 "/Game/Game/Obstacles/Materials/M_Red.M_Red")
      (set `self.Current Velocity` (/ (`self.MaxSpeed`) 5.0)))))

(fn `UserConstructionScript`)